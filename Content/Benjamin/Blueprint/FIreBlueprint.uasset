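; Fire projectile actor that moves its particle system along a forward vector and destroys itself after a set lifetime.
; Tick applies the speed-scaled offset without sweeping and also starts the lifetime delay that leads to destruction.
; Sphere hits on anything other than the player or its own class spawn an explosion at the particle's location, with debug prints, but do not destroy the projectile.
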(event OnComponentHit(Sphere)
  (params (HitComponent :type Primitive%20Component%20Object%20Reference) (OtherActor :type Actor%20Object%20Reference) (OtherComp :type Primitive%20Component%20Object%20Reference) (NormalImpulse :type Vector :default "0, 0, 0") (Hit :type Hit%20Result%20Structure%20%28by%20ref%29))
  (Development|PrintString "Try Collide")
  (if (and (!= OtherActor (Variables|Default|GetPlayer)) (!= (Utilities|GetClass OtherActor) (Utilities|GetClass self)))
    (Development|PrintString (Utilities|String|Append "Collided With " (Utilities|GetDisplayName OtherActor)))
    (Effects|SpawnEmitteratLocation "/Game/StarterContent/Particles/P_Explosion.P_Explosion" (Transformation|GetWorldLocation (Variables|Default|GetParticleSystem)))))

(event EventBeginPlay)

(event Collision|EventActorBeginOverlap
  (params (OtherActor :type Actor%20Object%20Reference)))

(event EventTick
  (params (DeltaSeconds :type Float%20%28single-precision%29))
  (Transformation|AddWorldOffset (Variables|Default|GetParticleSystem) (* (Variables|Default|GetForwardVector) (* DeltaSeconds (Variables|Default|GetMovementSpeed))) false false)
  (Utilities|FlowControl|Delay (Variables|Default|GetLifetime))
  (Actor|DestroyActor))

(fn ConstructionScript)